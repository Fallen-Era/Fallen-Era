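; Player controller that shows the build HUD for the local player and binds it to whichever pawn is possessed.
; BeginPlay listens for possessed-pawn changes and runs the handler once for the current pawn.
; For a valid pawn on a local controller, it creates WBP_BuildHud if needed and adds it to the viewport.
; It then injects MVVM view models, by class, from the pawn's build HUD and interaction prompt components.
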(event Custom|HandlePawnChanged
  (params (OldPawn :type Pawn%20Object%20Reference) (NewPawn :type Pawn%20Object%20Reference))
  (if (Pawn|IsLocalPlayerController)
    (Utilities|IsValid NewPawn
      (:Is%20Valid
        (Utilities|IsValid (Variables|Default|GetHudWidget)
          (:Is%20Valid
            _)
          (:Is%20Not%20Valid
            (bind _returnvalue (UserInterface|CreateWidget "/Game/Building/UI/WBP_BuildHud.WBP_BuildHud_C" self 0 0))
            (bind _output_get (Variables|Default|SetHudWidget _returnvalue))))
        (UserInterface|Viewport|AddtoViewport _output_get 0)
        (Class|MVVMBlueprintLibrary|SetViewModelbyClass (Variables|Default|GetHudWidget) (Class|FEBuildHudComponent|GetViewModel (Actor|GetComponentbyClass NewPawn "/Script/FallenEra.FEBuildHudComponent")))
        (Class|MVVMBlueprintLibrary|SetViewModelbyClass (Variables|Default|GetHudWidget) (Class|FEInteractionComponent|GetPromptViewModel (Actor|GetComponentbyClass NewPawn "/Script/FallenEra.FEInteractionComponent")))))))

(event EventBeginPlay
  (Pawn|BindEventtoOnPossessedPawnChanged (delegate Custom|HandlePawnChanged))
  (CallFunction|HandlePawnChanged 0 (Pawn|GetControlledPawn)))

(event EventTick
  (params (DeltaSeconds :type Float%20%28single-precision%29)))

(fn ConstructionScript)